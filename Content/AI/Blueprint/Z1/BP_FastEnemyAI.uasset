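; Fast enemy AI Blueprint that chases the player on sight and performs a melee-range attack animation.
; PawnSensing sets a seeing flag, never cleared here, and calls FollowPlayer, which runs AIMoveTo toward the player character.
; On arrival it plays a sped-up attack montage, using the returned length as a Delay before re-enabling CanAttack.
; Each FollowPlayer call also resets CanAttack, so a new sighting can bypass that gate.
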(event `self.PawnSensing.OnSeePawn`
  (params (Pawn :type "Pawn Object Reference"))
  (set `self.isSeeingPlayer?` true)
  (`self.FollowPlayer`))

(event `FollowPlayer`
  (set `self.CanAttack?` true)
  (if (`self.isSeeingPlayer?`)
    (`|AIMoveTo` self (0.0 0.0 0.0) (`GameplayStatics.GetPlayerCharacter` 0) 100.0
      (:`OnSuccess`
        (if (`self.CanAttack?`)
          (set `self.CanAttack?` false)
          (bind _returnvalue (`self.PlayAnimMontage` "/Game/AI/Animation/Montage/Anim_atk_Montage.Anim_atk_Montage" 2.0))
          (`KismetSystemLibrary.Delay` _returnvalue)
          (set `self.CanAttack?` true))))))

(fn `UserConstructionScript`)