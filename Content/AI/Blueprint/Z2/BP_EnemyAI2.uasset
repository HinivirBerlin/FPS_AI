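; Zombie enemy character that chases the player on sight, attacks in melee and awards score when shot or killed.
; PawnSensing sets a never-cleared seen flag and starts AI MoveTo; reaching the player plays an attack montage and applies damage, gated by CanAttack.
; Damage lowers Health and adds score; a hit arriving at zero Health or below plays death montage and sound, adds score, then destroys the actor.
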(event `self.ReceiveBeginPlay`
  (bind _asbp_player (cast `/Game/Blueprint/BP_Player` (`GameplayStatics.GetPlayerCharacter` 0)))
  (set `self.As BP Player` _asbp_player))

(event `self.PawnSensing.OnSeePawn`
  (params (Pawn :type "Pawn Object Reference"))
  (set `self.isSeeingPlayer?` true)
  (`self.FollowPlayer`))

(event `FollowPlayer`
  (set `self.CanAttack?` true)
  (if (`self.isSeeingPlayer?`)
    (`|AIMoveTo` self (0.0 0.0 0.0) (`self.As BP Player`) 100.0
      (:`OnSuccess`
        (if (`self.CanAttack?`)
          (set `self.CanAttack?` false)
          (bind _returnvalue (`self.PlayAnimMontage` "/Game/AI/Animation/Montage/Anim_atk_Montage.Anim_atk_Montage" 2.0))
          (`GameplayStatics.ApplyDamage` (`self.As BP Player`) 10.0)
          (`KismetSystemLibrary.Delay` _returnvalue)
          (set `self.CanAttack?` true))))))

(event `self.ReceiveAnyDamage`
  (params (Damage :type "Float (single-precision)") (DamageType :type "DamageType Object Reference") (InstigatedBy :type "Controller Object Reference") (DamageCauser :type "Actor Object Reference"))
  (bind _health (`self.Health`))
  (bind _as_bp_player (`self.As BP Player`))
  (if (> _health 0.0)
    (set `self.Health` (- _health Damage))
    (`/Game/Blueprint/BP_Player.Add score` _as_bp_player 5)
    (else
      (`|AIMoveTo` self (0.0 0.0 0.0) (`ActorComponent.GetOwner` (`self.Mesh`))
        (:`then`
          (`self.PlayAnimMontage` "/Game/AI/Animation/Montage/Anim_death_Montage.Anim_death_Montage")
          (`GameplayStatics.PlaySoundAtLocation` "/Game/AI/Zombie_death.Zombie_death" (`SceneComponent.K2_GetComponentLocation` (`self.Mesh`)) (struct) 1.0 1.0 0.0 null null null null)
          (`/Game/Blueprint/BP_Player.Add score` _as_bp_player 10)
          (`KismetSystemLibrary.Delay` 1.0)
          (`self.K2_DestroyActor`))))))

(fn `UserConstructionScript`)