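; Boss enemy spawner that starts spawning automatically on BeginPlay and keeps producing enemies on a repeating timer.
; StartSpawning sets an IsSpawning flag and starts a looping timer, bound by function name to SpawnZombie at the SpawnInterval rate.
; Each tick of that timer spawns a random class from the first four EnemyTypes entries at the Arrow component's world location.
; The graph contains no stop condition or spawn cap.
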(event `self.ReceiveBeginPlay`
  (`self.StartSpawning`))

(event `SpawnZombie`
  (`|SpawnActorFromClass` (`|GetArrayItem` (`self.EnemyTypes`) (`KismetMathLibrary.RandomIntegerInRange` 0 3)) (`KismetMathLibrary.MakeTransform` (`SceneComponent.K2_GetComponentLocation` (`self.Arrow`))) "Undefined" "MultiplyWithRoot" null null))

(event `StartSpawning`
  (set `self.IsSpawning` true)
  (`KismetSystemLibrary.K2_SetTimer` null "SpawnZombie" (`self.SpawnInterval`) true))

(fn `UserConstructionScript`)