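; Ammo vending machine that sells ammo for the player's current weapon in exchange for score.
; BeginPlay caches the player and creates a hidden WBP_Interact prompt, which the PickUpRadius overlap shows with weapon type and price, without checking the overlapping actor.
; Interact deducts Price from a sufficient Score, updates the HUD and adds a fixed ammo amount per weapon type.
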(event `/Game/Blueprint/Interface/BPI_Interact.Interact`
  (params (`Character Picking Up` :type "/Game/Blueprint/BP_Player Object Reference"))
  (bind _score (`/Game/Blueprint/BP_Player.Score` `Character Picking Up`))
  (bind _weapon_type (`/Game/Blueprint/Props/Weapon/BP_WeaponMaster.Weapon Type` (`/Game/Blueprint/BP_Player.Get Current Weapon` `Character Picking Up`)))
  (`KismetSystemLibrary.PrintString` "Hello")
  (if (>= _score (`self.price`))
    (bind _output_get (set `/Game/Blueprint/BP_Player.Score` (- _score (`self.price`)) `Character Picking Up`))
    (`/Game/Blueprint/Widget/WBP_HUD.Update Score TXT` (`/Game/Blueprint/BP_Player.HUDReff` `Character Picking Up`) _output_get)
    (switch `/Game/Blueprint/Props/Weapon/E_WeaponType` _weapon_type
      (:`NewEnumerator1`
        (`/Game/Blueprint/BP_Player.Adding Ammo` `Character Picking Up` 30 _weapon_type))
      (:`NewEnumerator2`
        (`/Game/Blueprint/BP_Player.Adding Ammo` `Character Picking Up` 18 _weapon_type))
      (:`NewEnumerator3`
        (`/Game/Blueprint/BP_Player.Adding Ammo` `Character Picking Up` 30 _weapon_type))
      (:`NewEnumerator4`
        (`/Game/Blueprint/BP_Player.Adding Ammo` `Character Picking Up` 5 _weapon_type)))))

(event `self.ReceiveBeginPlay`
  (bind _asbp_player (cast `/Game/Blueprint/BP_Player` (`GameplayStatics.GetPlayerCharacter` 0)))
  (set `self.As BP Player` _asbp_player)
  (bind _returnvalue (`|CreateWidget` "/Game/Blueprint/Widget/WBP_Interact.WBP_Interact_C"))
  (set `self.WBP_Interact` _returnvalue)
  (`UserWidget.AddToViewport` _returnvalue 0)
  (`Widget.SetVisibility` _returnvalue "Hidden")
  (`parent.ReceiveBeginPlay`))

(event `self.PickUp Radius.OnComponentBeginOverlap`
  (params (OverlappedComponent :type "PrimitiveComponent Object Reference") (OtherActor :type "Actor Object Reference") (OtherComp :type "PrimitiveComponent Object Reference") (OtherBodyIndex :type Integer) (bFromSweep :type Boolean) (SweepResult :type "HitResult Structure (by ref)"))
  (bind _wbp_interact (`self.WBP_Interact`))
  (bind _weapon_type (`/Game/Blueprint/Props/Weapon/BP_WeaponMaster.Weapon Type` (`/Game/Blueprint/BP_Player.Get Current Weapon` (`self.As BP Player`))))
  (switch `/Game/Blueprint/Props/Weapon/E_WeaponType` _weapon_type
    (:`NewEnumerator1`
      _)
    (:`NewEnumerator2`
      _)
    (:`NewEnumerator3`
      _)
    (:`NewEnumerator4`
      _))
  (`Widget.SetVisibility` _wbp_interact "Visible")
  (`/Game/Blueprint/Widget/WBP_Interact.Update Txt` _wbp_interact _weapon_type (`self.price`)))

(event `self.PickUp Radius.OnComponentEndOverlap`
  (params (OverlappedComponent :type "PrimitiveComponent Object Reference") (OtherActor :type "Actor Object Reference") (OtherComp :type "PrimitiveComponent Object Reference") (OtherBodyIndex :type Integer))
  (`Widget.SetVisibility` (`self.WBP_Interact`) "Hidden"))

(fn `UserConstructionScript`
  (`parent.UserConstructionScript`))