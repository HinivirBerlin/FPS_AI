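; Tutorial trigger box that shows an on-screen chat message when the player overlaps it.
; On overlap it removes the chat widget stored in BP_GlobalVar on the game instance, before checking that the actor is BP_Player.
; The Selection value picks the hint, from movement and combat basics to shield and ammo.
; CreateWidge spawns a timed WBP_ChatBox, which is saved back to BP_GlobalVar for the next trigger to clear.
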(event `self.Box.OnComponentBeginOverlap`
  (params (OverlappedComponent :type "PrimitiveComponent Object Reference") (OtherActor :type "Actor Object Reference") (OtherComp :type "PrimitiveComponent Object Reference") (OtherBodyIndex :type Integer) (bFromSweep :type Boolean) (SweepResult :type "HitResult Structure (by ref)"))
  (bind _returnvalue (`GameplayStatics.GetPlayerController` 0))
  (bind _as_bp_global_var (`self.As BP Global Var`))
  (bind _asbp_global_var (cast `/Game/Blueprint/BP_GlobalVar` (`GameplayStatics.GetGameInstance`)))
  (set `self.As BP Global Var` _asbp_global_var)
  (bind _bp_triggerbox_chat (`/Game/Blueprint/BP_GlobalVar.BP_TriggerBox_Chat` _asbp_global_var))
  (if (`KismetSystemLibrary.IsValid` _bp_triggerbox_chat)
    (`Widget.RemoveFromParent` _bp_triggerbox_chat))
  (cast `/Game/Blueprint/BP_Player` OtherActor)
  (switch `/Game/Blueprint/E_ChatBox` (`self.Selection`)
    (:`NewEnumerator0`
      (bind _returnvalue_2 (`self.CreateWidge` _returnvalue "You can move using forward, left, right and backward. The keys is set in the keybind window in the option menu." 5.0))
      (set `/Game/Blueprint/BP_GlobalVar.BP_TriggerBox_Chat` _returnvalue_2 _as_bp_global_var))
    (:`NewEnumerator1`
      (bind _returnvalue_3 (`self.CreateWidge` _returnvalue "You can jump using the jumping key and you also have a double jump just trigger the jump key in the air. The key is set in the keybind window in the option menu." 5.0))
      (set `/Game/Blueprint/BP_GlobalVar.BP_TriggerBox_Chat` _returnvalue_3 _as_bp_global_var))
    (:`NewEnumerator2`
      (bind _returnvalue_4 (`self.CreateWidge` _returnvalue "You can sprint using the sprint key. The key is set in the keybind window in the option menu." 5.0))
      (set `/Game/Blueprint/BP_GlobalVar.BP_TriggerBox_Chat` _returnvalue_4 _as_bp_global_var))
    (:`NewEnumerator3`
      (bind _returnvalue_5 (`self.CreateWidge` null "Look like you need to crunch to go further in this tutorial, use the crouch key set in your setting (base key is Ctrl)" 5.0))
      (set `/Game/Blueprint/BP_GlobalVar.BP_TriggerBox_Chat` _returnvalue_5 _as_bp_global_var))
    (:`NewEnumerator4`
      (bind _returnvalue_6 (`self.CreateWidge` null "A Zombie, take the gun and shoot that thing" 5.0))
      (set `/Game/Blueprint/BP_GlobalVar.BP_TriggerBox_Chat` _returnvalue_6 _as_bp_global_var))
    (:`NewEnumerator5`
      (bind _returnvalue_7 (`self.CreateWidge` null "Every time you get hit, you shield will be damage and when you shield break, you take damage on your health, be aware of that on the battlefield." 5.0))
      (set `/Game/Blueprint/BP_GlobalVar.BP_TriggerBox_Chat` _returnvalue_7 _as_bp_global_var))
    (:`NewEnumerator6`
      (bind _returnvalue_8 (`self.CreateWidge` null "You see this, it will give you back some shield. You don't need to worry about your health, it will regen with time." 5.0))
      (set `/Game/Blueprint/BP_GlobalVar.BP_TriggerBox_Chat` _returnvalue_8 _as_bp_global_var))
    (:`NewEnumerator7`
      (bind _returnvalue_9 (`self.CreateWidge` null "On the battlefield, you will find some ammo on the ground or maybe on one of this ammo dispenser, it will give you back some ammo on the weapon currently equip. " 5.0))
      (set `/Game/Blueprint/BP_GlobalVar.BP_TriggerBox_Chat` _returnvalue_9 _as_bp_global_var))
    (:`NewEnumerator8`
      (bind _returnvalue_10 (`self.CreateWidge` null "All the explanation are done, now grab those gun and shoot those bastard." 5.0))
      (set `/Game/Blueprint/BP_GlobalVar.BP_TriggerBox_Chat` _returnvalue_10 _as_bp_global_var))))

(fn `CreateWidge`
  (params (OwningPlayer :type "PlayerController Object Reference") (TextToDisplay :type String) (Time :type "Float (double-precision)") (isScreenLibre :type Boolean))
  (returns (ReturnValue :type "/Game/Blueprint/WBP_ChatBox Object Reference"))
  (bind _returnvalue (`|CreateWidget` "/Game/Blueprint/WBP_ChatBox.WBP_ChatBox_C" OwningPlayer TextToDisplay Time isScreenLibre))
  (`UserWidget.AddToViewport` _returnvalue 0)
  (return _returnvalue))

(fn `UserConstructionScript`)