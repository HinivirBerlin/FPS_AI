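; Boss enemy Blueprint with a health bar widget, melee-style attacks and a death sequence that leads to the end level.
; Attack plays one of two random montages, damaging the cached player as the montage starts rather than on a hit check, with a flag blocking overlap.
; Incoming damage updates the bar and awards score; at zero health it stops movement, plays Death, grants bonus score and opens L_End.
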(event `self.ReceiveBeginPlay`
  (bind _asbp_player (cast `/Game/Blueprint/BP_Player` (`GameplayStatics.GetPlayerCharacter` 0)))
  (set `self.As BP Player` _asbp_player)
  (bind _returnvalue (`|CreateWidget` "/Game/Boss/Blueprint/WB_BossHealth.WB_BossHealth_C"))
  (`UserWidget.AddToViewport` _returnvalue 0)
  (set `self.Health UI` _returnvalue))

(event `Actualize_life`
  (`ProgressBar.SetPercent` (`/Game/Boss/Blueprint/WB_BossHealth.HealthBar` (`self.Health UI`)) (/ (`self.Health`) 7500.0)))

(event `/Game/Boss/Behavior_tree/BPI_BossFight.Attack`
  (bind _as_bp_player (`self.As BP Player`))
  (bind _mesh (`self.Mesh`))
  ;[0.7057 0 0.02173 0.5] Attack
  (if (not (`self.IsAttacking`))
    (if (== (`KismetMathLibrary.RandomIntegerInRange` 0 1) 0)
      (`|PlayMontage` _mesh "/Game/Boss/Animation/Anim_compil/Montage/AM_Attack_One.AM_Attack_One"
        (:`then`
          (`GameplayStatics.ApplyDamage` _as_bp_player 20.0)
          (set `self.IsAttacking` true))
        (:`OnCompleted`
          (set `self.IsAttacking` false)))
      (else
        (`|PlayMontage` _mesh "/Game/Boss/Animation/Anim_compil/Montage/AM_Attack_Two.AM_Attack_Two"
          (:`then`
            (`GameplayStatics.ApplyDamage` _as_bp_player 20.0)
            (set `self.IsAttacking` true))
          (:`OnCompleted`
            (set `self.IsAttacking` false)))))))

(event `self.ReceiveAnyDamage`
  (params (Damage :type "Float (single-precision)") (DamageType :type "DamageType Object Reference") (InstigatedBy :type "Controller Object Reference") (DamageCauser :type "Actor Object Reference"))
  (bind _as_bp_player (`self.As BP Player`))
  ;[0 0.15 0.0251 0.5] Health System
  (set `self.Health` (- (`self.Health`) Damage))
  (`self.Actualize_life`)
  (`/Game/Blueprint/BP_Player.Add score` _as_bp_player 5)
  (if (<= (`self.Health`) 0.0)
    (`CharacterMovementComponent.DisableMovement` (`self.CharacterMovement`))
    (`|PlayMontage` (`self.Mesh`) "/Game/Boss/Animation/Anim_compil/Montage/Death.Death"
      (:`OnCompleted`
        (`/Game/Blueprint/BP_Player.Add score` _as_bp_player 50)
        (`self.K2_DestroyActor`)
        (`GameplayStatics.OpenLevelBySoftObjectPtr` "/Game/Level/L_End.L_End")))))

(event `Reset Rush`
  (set `self.bCanRush` true))

(fn `UserConstructionScript`)